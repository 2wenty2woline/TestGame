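; BP_InventoryItem is an inventory item actor that displays a shape and a score from its InventoryData.
; The construction script selects a sphere, cube or cylinder mesh by Type and writes Score to a text render.
; It also creates a dynamic M_BaseColor instance and sets its Color to a random entry from ColorObj.
; On EndPlay it spawns the NS_Explosion Niagara effect at its location.
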(event EventBeginPlay)

(event Collision|EventActorBeginOverlap
  (params (OtherActor :type Actor%20Object%20Reference)))

(event EventTick
  (params (DeltaSeconds :type Float%20%28single-precision%29)))

(event EventEndPlay
  (params (EndPlayReason :type EEndPlayReason%20Enum :default "Destroyed"))
  (Niagara|SpawnSystematLocation "/Game/Inventory/NS_Explosion.NS_Explosion" (Transformation|GetActorLocation)))

(fn ConstructionScript
  (bind _inventorydata (Variables|Default|GetInventoryData))
  ;[0.06125 0.06125 0.06125] Set Static Mesh
  (Components|StaticMesh|SetStaticMesh (Variables|Default|GetStaticMesh) (Utilities|Select :Index (.type _inventorydata) :SPHERE "/Engine/BasicShapes/Sphere.Sphere" :CUBE "/Engine/BasicShapes/Cube.Cube" :CYLINDER "/Engine/BasicShapes/Cylinder.Cylinder"))
  ;[0.06125 0.06125 0.06125] Set Score
  (Rendering|Components|TextRender|SetText (Variables|Default|GetTextRender) (Utilities|Text|ToText(Integer) (.score _inventorydata)))
  ;[0.06125 0.06125 0.06125] Set Color Material
  (bind _returnvalue (Rendering|Material|CreateDynamicMaterialInstance (Variables|Default|GetStaticMesh) 0 "/Game/Inventory/M_BaseColor.M_BaseColor" "None" :!class /Script/Engine.PrimitiveComponent))
  (Rendering|Material|SetVectorParameterValue _returnvalue "Color" (.OutItem (Utilities|Array|Random (Variables|Default|GetColor%20Obj))) :!class /Script/Engine.MaterialInstanceDynamic))